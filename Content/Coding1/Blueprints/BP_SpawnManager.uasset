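; Spawn manager that gathers every BP_Spawner in the level on BeginPlay and steps through them in a spawn event.
; When the index passes the end of the list, it shuffles the spawners and restarts from the first.
; Each step checks the current spawner's AutoSpawn flag: auto spawners advance the index with a spawn call, while others spawn, advance, then call spawn again after a delay.
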(event `self.ReceiveBeginPlay`
  (bind _outactors (`GameplayStatics.GetAllActorsOfClass` "/Game/Coding1/Blueprints/BP_Spawner.BP_Spawner_C")) ; Get all the spawners
  (set `self.Spawners` _outactors))

(event `Spawn a thing`
  (if (>= (`self.Index`) (`KismetArrayLibrary.Array_Length` (`self.Spawners`)))
    (`KismetArrayLibrary.Array_Shuffle` (`self.Spawners`))
    (set `self.Index` 0))
  (if (`/Game/Coding1/Blueprints/BP_Spawner.AutoSpawn` (`|GetArrayItem` (`self.Spawners`) (`self.Index`)))
    (`/Engine/EditorBlueprintResources/StandardMacros.IncrementInt` (`self.Index`)
      (:`  `
        (`self.Spawn a thing`)))
    (else
      (`self.Spawn a thing`)
      (`/Engine/EditorBlueprintResources/StandardMacros.IncrementInt` (`self.Index`)
        (:`  `
          (`KismetSystemLibrary.Delay` 5.0)
          (`self.Spawn a thing`))))))

(fn `UserConstructionScript`)