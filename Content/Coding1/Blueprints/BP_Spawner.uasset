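; BP_Spawner is a spawner actor that creates an instance of the TheThing class at its SpawnPoint component's world transform, skipping the spawn if it would collide.
; On BeginPlay it prints a status message and, if AutoSpawn is set, calls the SpawnTheThing event.
; While AutoSpawn stays true, that event re-calls itself after a fixed delay to form a repeating spawn loop.
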(event `self.ReceiveBeginPlay`
  (`KismetSystemLibrary.PrintText` "Spawner Active")
  (if (`self.AutoSpawn`)
    (`self.Spawn the Thing`)))

(event `Spawn the Thing`
  (`|SpawnActorFromClass` (`self.The thing`) (`SceneComponent.K2_GetComponentToWorld` (`self.SpawnPoint`)) "DontSpawnIfColliding" "MultiplyWithRoot" null null)
  (if (`self.AutoSpawn`)
    (`KismetSystemLibrary.Delay` 5.0)
    (`self.Spawn the Thing`)))

(fn `UserConstructionScript`)